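; BP_EnemySpawner is a manager that periodically spawns crows, flying crows, stickmen, wolves and foxes.
; Looping timers start on BeginPlay, with crows first and the other three types after a delay.
; Each spawn checks a current-versus-max count, shared by both crow types and not updated here.
; Spawns use random reachable navmesh points around the spawner, raised skyward for flying crows, except stickmen, which get no location.
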(event `self.ReceiveBeginPlay`
  (`KismetSystemLibrary.K2_SetTimerDelegate` (delegate `Spawn Event Crow`) 0.5 true)
  (`KismetSystemLibrary.K2_SetTimerDelegate` (delegate `Spawn Event FlyCrow`) 1.0 true)
  (`KismetSystemLibrary.Delay` 10.0)
  (`KismetSystemLibrary.K2_SetTimerDelegate` (delegate `Spawn Event Stickman`) 20.0 true)
  (`KismetSystemLibrary.K2_SetTimerDelegate` (delegate `Spawn Event Wolf`) 15.0 true)
  (`KismetSystemLibrary.K2_SetTimerDelegate` (delegate `Spawn Event Fox`) 10.0 true))

(event `Spawn Event Stickman`
  (if (< (`self.CurrentStickman`) (`self.MaxStickman`))
    (`|SpawnActorFromClass` "/Game/Enemies/BP_Enemy_Stickman.BP_Enemy_Stickman_C" (`KismetMathLibrary.MakeTransform` (0.0 0.0 0.0)) "Undefined" "MultiplyWithRoot" null null)))

(event `Spawn Event FlyCrow`
  (bind _skyvectorcrow (`self.SkyVectorCrow`))
  (bind _randomlocation (`NavigationSystemV1.K2_GetRandomReachablePointInRadius` (`self.K2_GetActorLocation`) 7000.0 null null))
  (if (< (`self.CurrentCrow`) (`self.MaxCrow`))
    (`KismetMathLibrary.Vector_Set` _skyvectorcrow (.x _randomlocation) (.y _randomlocation) 2000.0)
    (`|SpawnActorFromClass` "/Game/Enemies/Crow/BP_Crow_OnlyFly_Remaster.BP_Crow_OnlyFly_Remaster_C" (`KismetMathLibrary.MakeTransform` _skyvectorcrow) "Undefined" "MultiplyWithRoot" null null)))

(event `Spawn Event Crow`
  (if (< (`self.CurrentCrow`) (`self.MaxCrow`))
    (`|SpawnActorFromClass` "/Game/Enemies/Crow/BP_Enemy_Crow.BP_Enemy_Crow_C" (`KismetMathLibrary.MakeTransform` (`NavigationSystemV1.K2_GetRandomReachablePointInRadius` (`self.K2_GetActorLocation`) 7000.0 null null)) "Undefined" "MultiplyWithRoot" null null)))

(event `Spawn Event Wolf`
  (if (< (`self.CurrentWolf`) (`self.MaxWolf`))
    (`|SpawnActorFromClass` "/Game/Enemies/Wolf/BP_Enemy_Wolf.BP_Enemy_Wolf_C" (`KismetMathLibrary.MakeTransform` (`NavigationSystemV1.K2_GetRandomReachablePointInRadius` (`self.K2_GetActorLocation`) 7000.0 null null)) "Undefined" "MultiplyWithRoot" null null)))

(event `Spawn Event Fox`
  (if (< (`self.CurrentFox`) (`self.MaxFox`))
    (`|SpawnActorFromClass` "/Game/Enemies/BP_Enemy_Fox.BP_Enemy_Fox_C" (`KismetMathLibrary.MakeTransform` (`NavigationSystemV1.K2_GetRandomReachablePointInRadius` (`self.K2_GetActorLocation`) 7000.0 null null)) "Undefined" "MultiplyWithRoot" null null)))

(fn `UserConstructionScript`)