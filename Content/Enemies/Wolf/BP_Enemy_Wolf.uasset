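; BP_Enemy_Wolf is a wolf enemy Blueprint that implements the Attack event for damaging the player.
; Attack randomly plays one of two montages on the mesh, AttackMontage or AM_Wolf_Attack2.
; Completion or interruption of either montage calls OnAttackEnd, then applies fixed damage to player pawn 0 without a range or hit check.
; The construction script only runs the parent's version.
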(event `self.Attack`
  (bind _mesh (`self.Mesh`))
  (if (`KismetMathLibrary.RandomBool`)
    (`|PlayMontage` _mesh (`self.AttackMontage`)
      (:`OnCompleted`
        _)
      (:`OnInterrupted`
        _))
    (else
      (`|PlayMontage` _mesh "/Game/AnimalVarietyPack/Wolf/Animations/AM_Wolf_Attack2.AM_Wolf_Attack2"
        (:`OnCompleted`
          _)
        (:`OnInterrupted`
          _))))
  (`self.OnAttackEnd`)
  (`GameplayStatics.ApplyDamage` (`GameplayStatics.GetPlayerPawn` 0) 20.0 null null "/Script/Engine.DamageType"))

(fn `UserConstructionScript`
  (`parent.UserConstructionScript`))