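; Stickman enemy character that stays dormant for the first 20 seconds after it begins play.
; After the parent BeginPlay, it disables movement, clears its AI controller class and behavior tree, and turns off visibility, collision and tick.
; A fixed delay then restores walking and those actor states, and assigns BT_Enemy_Stickman and AIC_Enemy_Base, with no explicit controller spawn or tree start here.
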(event `self.ReceiveBeginPlay`
  (`parent.ReceiveBeginPlay`)
  (`CharacterMovementComponent.SetMovementMode` (`self.CharacterMovement`) "MOVE_None" 0)
  (set `self.AIControllerClass` null)
  (set `self.BehaviorTree` null)
  (`self.SetActorHiddenInGame` true)
  (`self.SetActorEnableCollision` false)
  (`self.SetActorTickEnabled` false)
  (`KismetSystemLibrary.Delay` 20.0)
  (`CharacterMovementComponent.SetMovementMode` (`self.CharacterMovement`) "MOVE_Walking" 0)
  (set `self.BehaviorTree` "/Game/Enemies/AI/BehaviorTrees/BT_Enemy_Stickman.BT_Enemy_Stickman")
  (set `self.AIControllerClass` "/Game/Enemies/AI/AIC_Enemy_Base.AIC_Enemy_Base_C")
  (`self.SetActorHiddenInGame` false)
  (`self.SetActorEnableCollision` true)
  (`self.SetActorTickEnabled` true))

(event `self.ReceiveTick`
  (params (DeltaSeconds :type "Float (single-precision)")))

(fn `UserConstructionScript`
  (`parent.UserConstructionScript`))