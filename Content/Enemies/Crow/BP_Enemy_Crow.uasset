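; Crow enemy that takes damage, dies in the air or on the ground, and awards score to the first-person player.
; Damage plays a random sound and lowers health; non-lethal hits pause movement during the hit montage.
; Death starts a timed lifespan and plays either a ground death or, if flying, a switch to falling.
; Tick detects the dead crow landing, plays the impact montage, then disables collision and movement.
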(event `self.ReceiveBeginPlay`
  (`parent.ReceiveBeginPlay`))

(event `self.ReceiveTick`
  (params (DeltaSeconds :type "Float (single-precision)"))
  ; When he is dead and falls, play an impact animation when he touches the ground.
  (if (`self.isDead`)
    (if (`NavMovementInterface.IsFalling` (`self.CharacterMovement`))
      _
      (elif (not (`self.DeathOnGround`))
        (`|PlayMontage` (`self.Mesh`) "/Game/AnimalVarietyPack/Crow/Animations/AM_Crow_DeathHitGround.AM_Crow_DeathHitGround"
          (:`OnCompleted`
            _)
          (:`OnInterrupted`
            _))
        (set `self.DeathOnGround` true)
        (`PrimitiveComponent.SetCollisionEnabled` (`self.CapsuleComponent`) "NoCollision")
        (`CharacterMovementComponent.DisableMovement` (`self.CharacterMovement`))))))

(event `self.ReceiveAnyDamage`
  (params (Damage :type "Float (single-precision)") (DamageType :type "DamageType Object Reference") (InstigatedBy :type "Controller Object Reference") (DamageCauser :type "Actor Object Reference"))
  (bind _returnvalue (`self.K2_GetActorLocation`))
  (bind _charactermovement (`self.CharacterMovement`))
  (bind _charactermovement_2 (`self.CharacterMovement`))
  ; Play one of 2 random sounds
  (if (not (`self.isDead`))
    (if (`KismetMathLibrary.RandomBool`)
      (`GameplayStatics.SpawnSoundAtLocation` "/Game/Audio/Crow/Crow_Dmg_3.Crow_Dmg_3" _returnvalue (struct) 1.0 1.0 0.0 null null)
      (else
        (`GameplayStatics.SpawnSoundAtLocation` "/Game/Audio/Crow/Crow_Dmg_2.Crow_Dmg_2" _returnvalue (struct) 1.0 1.0 0.0 null null)))
    (bind _output_get (set `self.Health` (`KismetMathLibrary.FClamp` (- (`self.Health`) Damage) 0.0 (`self.MaxHealth`))))
    (if (<= _output_get 0.0)
      (set `self.isDead` true)
      (`self.SetLifeSpan` 10.0)
      ; When he flies, play a fall animation, otherwise play a death animation directly.
      (if (`NavMovementInterface.IsFlying` _charactermovement_2)
        (`NavMovementInterface.StopActiveMovement` _charactermovement_2)
        (`self.PlayAnimMontage` "/Game/AnimalVarietyPack/Crow/Animations/AM_Falling.AM_Falling")
        (`CharacterMovementComponent.SetMovementMode` (`self.CharacterMovement`) "MOVE_Falling" 0)
        (else
          (`self.PlayAnimMontage` "/Game/AnimalVarietyPack/Crow/Animations/AM_DeathGround_Crow.AM_DeathGround_Crow")))
      (bind _asbp_first_person_character (cast `/Game/FirstPerson/Blueprints/BP_FirstPersonCharacter` (`GameplayStatics.GetPlayerCharacter` 0)))
      (set `/Game/FirstPerson/Blueprints/BP_FirstPersonCharacter.Score` (+ (`/Game/FirstPerson/Blueprints/BP_FirstPersonCharacter.Score` _asbp_first_person_character) (`self.Points`)) _asbp_first_person_character)
      (else
        ; Hit Logic
        (`ActorComponent.Deactivate` _charactermovement)
        (bind _returnvalue_2 (`self.PlayAnimMontage` (`self.HitMontage`)))
        (`KismetSystemLibrary.Delay` _returnvalue_2)
        (`ActorComponent.Activate` _charactermovement false)))))

(fn `UserConstructionScript`
  (`parent.UserConstructionScript`))