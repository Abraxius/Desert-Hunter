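; Flying crow target that follows a spline path and awards points to the first-person player when shot.
; Tick advances a distance by speed and moves the Empty component along the spline, optionally looping.
; A projectile hit stops flight, plays a death montage, disables sphere collision, adds points and sets a one-second lifespan.
; Destroyed adds points again; the construction script's spline-segment loop is empty.
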(event `self.ReceiveHit`
  (params (MyComp :type "PrimitiveComponent Object Reference") (Other :type "Actor Object Reference") (OtherComp :type "PrimitiveComponent Object Reference") (bSelfMoved :type Boolean) (HitLocation :type "Vector Structure") (HitNormal :type "Vector Structure") (NormalImpulse :type "Vector Structure") (Hit :type "HitResult Structure (by ref)"))
  (cast `/Game/FirstPerson/Blueprints/BP_FirstPersonProjectile` Other)
  (if (not (`self.isDead`))
    (`self.SetLifeSpan` 1.0)
    (set `self.isDead` true)
    (`|PlayMontage` (`self.Crow`) "/Game/AnimalVarietyPack/Crow/Animations/AM_Crow_DeathHitGround.AM_Crow_DeathHitGround"
      (:`then`
        (bind _asbp_first_person_character (cast `/Game/FirstPerson/Blueprints/BP_FirstPersonCharacter` (`GameplayStatics.GetPlayerCharacter` 0)))
        (set `/Game/FirstPerson/Blueprints/BP_FirstPersonCharacter.Score` (+ (`/Game/FirstPerson/Blueprints/BP_FirstPersonCharacter.Score` _asbp_first_person_character) (`self.Points`)) _asbp_first_person_character)
        (`PrimitiveComponent.SetCollisionEnabled` (`self.Sphere`) "NoCollision")))))

(event `self.ReceiveTick`
  (params (DeltaSeconds :type "Float (single-precision)"))
  (bind (_returnvalue_location _returnvalue_rotation) (`KismetMathLibrary.BreakTransform` (`SplineComponent.GetTransformAtDistanceAlongSpline` (`self.Spline`) (`self.Distance`) "Local" false)))
  (if (not (`self.isDead`))
    (set `self.Distance` (+ (* DeltaSeconds (`self.Speed`)) (`self.Distance`) 1.0))
    (`SceneComponent.K2_SetRelativeTransform` (`self.Empty`) (`KismetMathLibrary.MakeTransform` _returnvalue_location _returnvalue_rotation (`SceneComponent.RelativeScale3D` (`self.Empty`))) false false)
    (if (`self.Islooping`)
      (if (> (`self.Distance`) (`SplineComponent.GetSplineLength` (`self.Spline`)))
        (set `self.Distance` 1.0)))))

(event `self.ReceiveDestroyed`
  (bind _asbp_first_person_character (cast `/Game/FirstPerson/Blueprints/BP_FirstPersonCharacter` (`GameplayStatics.GetPlayerCharacter` 0)))
  (set `/Game/FirstPerson/Blueprints/BP_FirstPersonCharacter.Score` (+ (`/Game/FirstPerson/Blueprints/BP_FirstPersonCharacter.Score` _asbp_first_person_character) (`self.Points`)) _asbp_first_person_character))

(fn `UserConstructionScript`
  (for _index (range (`KismetMathLibrary.FTrunc` (/ (`SplineComponent.GetSplineLength` (`self.Spline`)) (`self.Length`))))
    _))