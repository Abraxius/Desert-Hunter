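; Flying crow enemy that follows an external spline, optionally looping, and awards points to the player when shot down or destroyed.
; BeginPlay registers it in the enemy spawner's crow count, and Tick advances it along the spline by distance.
; Any damage switches it to falling with montage, sound, score and a timed lifespan, then Tick plays a ground-impact montage on landing.
; Destruction removes its spline actor and adds the points again.
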(event `self.ReceiveBeginPlay`
  (`CharacterMovementComponent.SetMovementMode` (`self.CharacterMovement`) "MOVE_Flying" 0)
  (bind _returnvalue (`GameplayStatics.GetActorOfClass` "/Game/Managers/BP_EnemySpawner.BP_EnemySpawner_C"))
  (set `/Game/Managers/BP_EnemySpawner.CurrentCrow` (+ (`/Game/Managers/BP_EnemySpawner.CurrentCrow` _returnvalue) 1) _returnvalue))

(event `self.ReceiveAnyDamage`
  (params (Damage :type "Float (single-precision)") (DamageType :type "DamageType Object Reference") (InstigatedBy :type "Controller Object Reference") (DamageCauser :type "Actor Object Reference"))
  (bind _returnvalue (`SceneComponent.K2_GetComponentLocation` (`self.Empty`)))
  (if (not (`self.isDead`))
    (`self.SetLifeSpan` 10.0)
    (`CharacterMovementComponent.SetMovementMode` (`self.CharacterMovement`) "MOVE_Falling" 0)
    (set `self.isDead` true)
    (`|PlayMontage` (`self.Crow`) "/Game/AnimalVarietyPack/Crow/Animations/AM_Falling.AM_Falling"
      (:`then`
        (bind _asbp_first_person_character (cast `/Game/FirstPerson/Blueprints/BP_FirstPersonCharacter` (`GameplayStatics.GetPlayerCharacter` 0)))
        (set `/Game/FirstPerson/Blueprints/BP_FirstPersonCharacter.Score` (+ (`/Game/FirstPerson/Blueprints/BP_FirstPersonCharacter.Score` _asbp_first_person_character) (`self.Points`)) _asbp_first_person_character)
        (`PrimitiveComponent.SetCollisionEnabled` (`self.Sphere`) "NoCollision")
        (if (`KismetMathLibrary.RandomBool`)
          (`GameplayStatics.SpawnSoundAtLocation` "/Game/Audio/Crow/Crow_Dmg_1.Crow_Dmg_1" _returnvalue (struct) 1.0 1.0 0.0 null null)
          (else
            (`GameplayStatics.SpawnSoundAtLocation` "/Game/Audio/Crow/Crow_Dmg_2.Crow_Dmg_2" _returnvalue (struct) 1.0 1.0 0.0 null null)))))))

(event `self.ReceiveHit`
  (params (MyComp :type "PrimitiveComponent Object Reference") (Other :type "Actor Object Reference") (OtherComp :type "PrimitiveComponent Object Reference") (bSelfMoved :type Boolean) (HitLocation :type "Vector Structure") (HitNormal :type "Vector Structure") (NormalImpulse :type "Vector Structure") (Hit :type "HitResult Structure (by ref)")))

(event `self.ReceiveTick`
  (params (DeltaSeconds :type "Float (single-precision)"))
  (bind (_returnvalue_location _returnvalue_rotation) (`KismetMathLibrary.BreakTransform` (`SplineComponent.GetTransformAtDistanceAlongSpline` (`self.ExtSpline`) (`self.Distance`) "World" false)))
  (if (`self.isDead`)
    (if (`NavMovementInterface.IsFalling` (`self.CharacterMovement`))
      _
      (elif (not (`self.DeathOnGround`))
        (`|PlayMontage` (`self.Crow`) "/Game/AnimalVarietyPack/Crow/Animations/AM_Crow_DeathHitGround.AM_Crow_DeathHitGround"
          (:`OnCompleted`
            _)
          (:`OnInterrupted`
            _))
        (set `self.DeathOnGround` true)))
    (else
      (set `self.Distance` (+ (* DeltaSeconds (`self.Speed`)) (`self.Distance`) 1.0))
      (`SceneComponent.K2_SetRelativeTransform` (`self.CapsuleComponent`) (`KismetMathLibrary.MakeTransform` _returnvalue_location _returnvalue_rotation) false false)
      (if (`self.Islooping`)
        (if (> (`self.Distance`) (`SplineComponent.GetSplineLength` (`self.ExtSpline`)))
          (set `self.Distance` 1.0))))))

(event `self.ReceiveDestroyed`
  (`self.K2_DestroyActor` (`self.SplineActor`))
  (bind _asbp_first_person_character (cast `/Game/FirstPerson/Blueprints/BP_FirstPersonCharacter` (`GameplayStatics.GetPlayerCharacter` 0)))
  (set `/Game/FirstPerson/Blueprints/BP_FirstPersonCharacter.Score` (+ (`/Game/FirstPerson/Blueprints/BP_FirstPersonCharacter.Score` _asbp_first_person_character) (`self.Points`)) _asbp_first_person_character))

(fn `UserConstructionScript`)